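; BP_PersonalityComponent is a component that stores a character's personality for the strategy simulator's character creator.
; SetPersonality builds a FCharacterPersonality struct from name, surname, sex, age, icon, stats, and favorite and least favorite jobs, then stores it in Personality.
; On BeginPlay it waits briefly, then prints the name, sex, age and icon name on screen as debug output.
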(event `self.ReceiveBeginPlay`
  (bind (_firstname _surname _sex _age _icon) (break `/Game/StratagySimulator/CharacterCreator/Structs/F_CharacterPersonality` (`self.Personality`)))
  (`KismetSystemLibrary.Delay` 5.0)
  (`KismetSystemLibrary.PrintString` (`KismetTextLibrary.Conv_TextToString` (`|FormatText` "{1} {2} {3} {4} years old ||||| Icon name: {5}" _firstname _surname (`|GetEnumeratorNameAsString` _sex) _age (`KismetSystemLibrary.GetDisplayName` _icon))) true true (struct :`G` 0.66 :`B` 1.0 :`A` 1.0) 50.0))

(fn `SetPersonality`
  (params (Name :type Text) (Surname :type Text) (Sex :type "/Game/StratagySimulator/CharacterCreator/Enums/E_Sex Enum" :default "NewEnumerator0") (Age :type Integer) (Icon :type "Texture2D Object Reference") (Stats :type "Map of GameplayTag Structure to Integer") (FavoriteJob :type "GameplayTagContainer Structure") (LeastFavoriteJob :type "GameplayTagContainer Structure"))
  (set `self.Personality` (make `/Game/StratagySimulator/CharacterCreator/Structs/F_CharacterPersonality` Name Surname Sex Age Icon Stats FavoriteJob LeastFavoriteJob)))