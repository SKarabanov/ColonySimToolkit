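; Spawner actor that creates a batch of randomized BP_Citizen characters scattered around its location on BeginPlay.
; Each citizen's personality receives a random sex, age, stats and non-overlapping favorite and least-favorite job tags drawn from the attribute keys.
; Names, surnames and icons come from random DataTable rows, with first names and icons split by sex.
; Stat points are distributed over shuffled attributes with a per-stat cap, recursing until the budget is spent.
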(event `self.ReceiveBeginPlay`
  (for _ (range 11)
    (`self.GenerateRandomCharacter`)))

(fn `GenerateCharacterName`
  (params (Sex :type "/Game/StratagySimulator/CharacterCreator/Enums/E_Sex Enum" :default "NewEnumerator0"))
  (returns (Name :type Text) (Surname :type Text))
  (locals (L_FirstName :type Text))
  (`|ExecutionSequence`
    (:`then_0`
      (switch `/Game/StratagySimulator/CharacterCreator/Enums/E_Sex` Sex
        (:`NewEnumerator0`
          (bind _outrownames (`DataTableFunctionLibrary.GetDataTableRowNames` "/Game/StratagySimulator/CharacterCreator/Tables/DT_MaleNames.DT_MaleNames"))
          (bind _returnvalue (`|GetDataTableRow` "/Game/StratagySimulator/CharacterCreator/Tables/DT_MaleNames.DT_MaleNames" (`KismetArrayLibrary.Array_Random` _outrownames))
            (:`then`
              (set `local.L_FirstName` (`.Name_2_4E877DD4404E3FFA88A3DBB6AD22C4A8` (break `/Game/StratagySimulator/CharacterCreator/Structs/F_NameData` _returnvalue))))))
        (:`NewEnumerator1`
          (bind _outrownames_2 (`DataTableFunctionLibrary.GetDataTableRowNames` "/Game/StratagySimulator/CharacterCreator/Tables/DT_FemaleNames.DT_FemaleNames"))
          (bind _returnvalue_2 (`|GetDataTableRow` "/Game/StratagySimulator/CharacterCreator/Tables/DT_FemaleNames.DT_FemaleNames" (`KismetArrayLibrary.Array_Random` _outrownames_2))
            (:`then`
              (set `local.L_FirstName` (`.Name_2_4E877DD4404E3FFA88A3DBB6AD22C4A8` (break `/Game/StratagySimulator/CharacterCreator/Structs/F_NameData` _returnvalue_2))))))))
    (:`then_1`
      (bind _outrownames_3 (`DataTableFunctionLibrary.GetDataTableRowNames` "/Game/StratagySimulator/CharacterCreator/Tables/DT_Surnames.DT_Surnames"))
      (bind _returnvalue_3 (`|GetDataTableRow` "/Game/StratagySimulator/CharacterCreator/Tables/DT_Surnames.DT_Surnames" (`KismetArrayLibrary.Array_Random` _outrownames_3))
        (:`then`
          (return (`local.L_FirstName`) (`.Name_2_4E877DD4404E3FFA88A3DBB6AD22C4A8` (break `/Game/StratagySimulator/CharacterCreator/Structs/F_NameData` _returnvalue_3))))))))

(fn `GenerateCharacterStats`
  (params (Attributes :type "Map of GameplayTag Structure to Integer (by ref)") (PointsAmount :type Integer) (bMinimumOnePoint :type Boolean :default true))
  (returns (Stats :type "Map of GameplayTag Structure to Integer"))
  (locals (L_Stats :type "Map of GameplayTag Structure to Integer") (L_Points :type Integer :default 0) (L_CurrentStatPoints :type Integer) (L_StatKeys :type "Array of GameplayTag Structure"))
  (set `local.L_Stats` Attributes)
  (set `local.L_Points` (`KismetMathLibrary.SelectInt` (- PointsAmount (`BlueprintMapLibrary.Map_Length` (`local.L_Stats`))) (`local.PointsAmount`) (`local.bMinimumOnePoint`)))
  (bind _keys (`BlueprintMapLibrary.Map_Keys` (`local.L_Stats`)))
  (bind _output_get (set `local.L_StatKeys` _keys))
  (`KismetArrayLibrary.Array_Shuffle` _output_get)
  (for _array_element (`local.L_StatKeys`)
    (if (> (`local.L_Points`) 0)
      (bind _value (`BlueprintMapLibrary.Map_Find` (`local.L_Stats`) _array_element))
      (bind _output_get_2 (set `local.L_CurrentStatPoints` (`KismetMathLibrary.RandomIntegerInRange` 0 (`KismetMathLibrary.Min` (- 10 _value) (`local.L_Points`)))))
      (`BlueprintMapLibrary.Map_Add` (`local.L_Stats`) _array_element (+ _output_get_2 _value))
      (set `local.L_Points` (- (`local.L_Points`) (`local.L_CurrentStatPoints`)))
      (else
        (return (`local.L_Stats`)))))
  (if (> (`local.L_Points`) 0)
    (bind _stats (`self.GenerateCharacterStats` (`local.L_Stats`) (`local.L_Points`) false))
    (return _stats)
    (else
      (return (`local.L_Stats`)))))

(fn `GenerateIcon`
  (params (Sex :type "/Game/StratagySimulator/CharacterCreator/Enums/E_Sex Enum" :default "NewEnumerator0"))
  (returns (Icon :type "Texture2D Object Reference"))
  (switch `/Game/StratagySimulator/CharacterCreator/Enums/E_Sex` Sex
    (:`NewEnumerator0`
      (bind _outrownames (`DataTableFunctionLibrary.GetDataTableRowNames` "/Game/StratagySimulator/CharacterCreator/Tables/DT_CharacterIcons_Male.DT_CharacterIcons_Male"))
      (bind _returnvalue (`|GetDataTableRow` "/Game/StratagySimulator/CharacterCreator/Tables/DT_CharacterIcons_Male.DT_CharacterIcons_Male" (`KismetArrayLibrary.Array_Random` _outrownames))
        (:`then`
          (return (`.Icon_3_015EC1D14880A4FA3DD2D19D60F55858` (break `/Game/StratagySimulator/CharacterCreator/Structs/F_CharacterIcon` _returnvalue))))))
    (:`NewEnumerator1`
      (bind _outrownames_2 (`DataTableFunctionLibrary.GetDataTableRowNames` "/Game/StratagySimulator/CharacterCreator/Tables/DT_CharacterIcons_Female.DT_CharacterIcons_Female"))
      (bind _returnvalue_2 (`|GetDataTableRow` "/Game/StratagySimulator/CharacterCreator/Tables/DT_CharacterIcons_Female.DT_CharacterIcons_Female" (`KismetArrayLibrary.Array_Random` _outrownames_2))
        (:`then`
          (return (`.Icon_3_015EC1D14880A4FA3DD2D19D60F55858` (break `/Game/StratagySimulator/CharacterCreator/Structs/F_CharacterIcon` _returnvalue_2))))))))

(fn `GenerateRandomCharacter`
  (locals (L_Sex :type "/Game/StratagySimulator/CharacterCreator/Enums/E_Sex Enum") (L_Personality :type "/Game/StratagySimulator/CharacterCreator/Blueprints/BP_PersonalityComponent Object Reference") (L_Attributes :type "Map of GameplayTag Structure to Integer") (L_FavoriteTags :type "GameplayTagContainer Structure") (L_LeastFavoriteTags :type "GameplayTagContainer Structure") (L_Tag :type "GameplayTag Structure"))
  (bind _returnvalue (`KismetMathLibrary.RandomFloatInRange` -1000.0 1000.0))
  (bind (_agelimit_minimumage _agelimit_maximumage) (break `/Game/StratagySimulator/CharacterCreator/Structs/F_AgeLimit` (`self.AgeLimit`)))
  (bind _returnvalue_2 (`|SpawnActorFromClass` "/Game/StratagySimulator/CharacterCreator/Blueprints/BP_Citizen.BP_Citizen_C" (`KismetMathLibrary.MakeTransform` (`KismetMathLibrary.MakeVector` (+ (.x (`self.K2_GetActorLocation`)) _returnvalue) (+ _returnvalue (.y (`self.K2_GetActorLocation`))) (.z (`self.K2_GetActorLocation`)))) "AlwaysSpawn" "MultiplyWithRoot" null null))
  (bind _result (message `/Game/StratagySimulator/CharacterCreator/Blueprints/BPI_Character.GetPersonality` _returnvalue_2))
  (bind _output_get (set `local.L_Personality` _result))
  (`/Engine/EditorBlueprintResources/StandardMacros.IsValid` _output_get
    (:`Is Valid`
      (bind _stats (`self.GenerateCharacterStats` (`self.CharacterAttributes`) (`self.StartPointsAmount`)))
      (set `local.L_Attributes` _stats)
      (if (> (`self.FavoriteJobAmount`) 0)
        (for _ (range 1 (+ (`self.FavoriteJobAmount`) 1))
          (bind _keys (`BlueprintMapLibrary.Map_Keys` (`local.L_Attributes`)))
          (bind _output_get_2 (set `local.L_Tag` (`KismetArrayLibrary.Array_Random` _keys)))
          (`BlueprintGameplayTagLibrary.AddGameplayTag` (`local.L_FavoriteTags`) _output_get_2)
          (`BlueprintMapLibrary.Map_Remove` (`local.L_Attributes`) (`local.L_Tag`))))
      (if (> (`self.LeastFavoriteJobAmount`) 0)
        (for _ (range 1 (+ (`self.LeastFavoriteJobAmount`) 1))
          (bind _keys_2 (`BlueprintMapLibrary.Map_Keys` (`local.L_Attributes`)))
          (bind _output_get_3 (set `local.L_Tag` (`KismetArrayLibrary.Array_Random` _keys_2)))
          (`BlueprintGameplayTagLibrary.AddGameplayTag` (`local.L_LeastFavoriteTags`) _output_get_3)
          (`BlueprintMapLibrary.Map_Remove` (`local.L_Attributes`) (`local.L_Tag`))))
      (bind _output_get_4 (set `local.L_Sex` (cast `/Game/StratagySimulator/CharacterCreator/Enums/E_Sex` (`KismetMathLibrary.Conv_IntToByte` (`KismetMathLibrary.RandomIntegerInRange` 0 (- (enumcount `/Game/StratagySimulator/CharacterCreator/Enums/E_Sex`) 1))))))
      (bind (_name _surname) (`self.GenerateCharacterName` _output_get_4))
      (`/Game/StratagySimulator/CharacterCreator/Blueprints/BP_PersonalityComponent.SetPersonality` (`local.L_Personality`) _name _surname (`local.L_Sex`) (`KismetMathLibrary.RandomIntegerInRange` _agelimit_minimumage _agelimit_maximumage) (`self.GenerateIcon` (`local.L_Sex`)) _stats (`local.L_FavoriteTags`) (`local.L_LeastFavoriteTags`)))))

(fn `UserConstructionScript`)