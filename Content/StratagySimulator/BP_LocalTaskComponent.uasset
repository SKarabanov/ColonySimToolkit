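; BP_LocalTaskComponent is a component that holds its owner's current task and an editable priority map of types to values.
; TakeTask stores the current task and ChangePriority writes a value into the map.
; GetSortedPriorityArray orders keys from highest to lowest value by repeatedly taking the maximum and overwriting it with -1.
; Its index check only accepts maxima above index zero, so the first entry is never added.
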(event `self.ReceiveBeginPlay`)

(fn `ChangePriority`
  (params (Type :type "/Game/StratagySimulator/Blueprints/Data/Enums/E_TaskType Enum (by ref)") (Value :type "Integer (by ref)"))
  (`BlueprintMapLibrary.Map_Add` (`self.PriorityList`) Type Value))

(fn `GetSortedPriorityArray`
  (returns (result :type "Array of /Game/StratagySimulator/Blueprints/Data/Enums/E_TaskType Enum"))
  (locals (L_ValueArray :type "Array of Integer") (L_SortedKeyArray :type "Array of /Game/StratagySimulator/Blueprints/Data/Enums/E_TaskType Enum"))
  (bind _indexofmaxvalue (`KismetMathLibrary.MaxOfIntArray` (`local.L_ValueArray`)))
  (bind _values (`BlueprintMapLibrary.Map_Values` (`self.PriorityList`)))
  (bind _output_get (set `local.L_ValueArray` _values))
  (bind _keys (`BlueprintMapLibrary.Map_Keys` (`self.PriorityList`)))
  (for _ (range (+ (`KismetArrayLibrary.Array_LastIndex` _output_get) 1))
    (if (> _indexofmaxvalue 0)
      (`KismetArrayLibrary.Array_Add` (`local.L_SortedKeyArray`) (`|GetArrayItem` _keys _indexofmaxvalue))
      (`KismetArrayLibrary.Array_Set` (`local.L_ValueArray`) _indexofmaxvalue -1)))
  (return (`local.L_SortedKeyArray`)))

(fn `TakeTask`
  (params (NewTask :type "/Game/StratagySimulator/BP_Task_Base Object Reference"))
  (set `self.CurrentTask` NewTask))