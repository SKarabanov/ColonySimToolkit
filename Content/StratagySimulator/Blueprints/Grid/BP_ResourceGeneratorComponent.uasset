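; Component on a BP_TerrainGenerator that scatters resource container actors over the instanced-block terrain.
; GenerateResources clears tracked containers, calls FillBiomes, then picks unused random cells for each class and count in the Resources map.
; Debug-drawn sphere traces find the hit terrain instance, and a randomly yawed container spawns on its top.
; BeginPlay separately runs a delayed, hardcoded scatter of untracked wood containers, randomizing trace start and end independently.
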(event `self.ReceiveBeginPlay`
  (`KismetSystemLibrary.Delay` 2.0)
  (bind _asbp_terrain_generator (cast `/Game/StratagySimulator/Blueprints/Grid/BP_TerrainGenerator` (`self.GetOwner`)))
  (for _ (range 31)
    (bind _returnvalue (`Actor.K2_GetActorLocation` _asbp_terrain_generator))
    (bind (_fragmentsize_x _fragmentsize_y _fragmentsize_z) (`KismetMathLibrary.BreakVector` (`/Game/StratagySimulator/Blueprints/Grid/BP_TerrainGenerator.FragmentSize` _asbp_terrain_generator)))
    (bind _returnvalue_2 (* (`KismetMathLibrary.RandomIntegerInRange` 0 (`/Game/StratagySimulator/Blueprints/Grid/BP_TerrainGenerator.Width` _asbp_terrain_generator)) _fragmentsize_x))
    (bind _returnvalue_3 (* (`KismetMathLibrary.RandomIntegerInRange` 0 (`/Game/StratagySimulator/Blueprints/Grid/BP_TerrainGenerator.Length` _asbp_terrain_generator)) _fragmentsize_y))
    (bind (_outhits _returnvalue_4) (`KismetSystemLibrary.SphereTraceMulti` :`Start` (+ _returnvalue (`KismetMathLibrary.MakeVector` _returnvalue_2 _returnvalue_3 (* (+ (`/Game/StratagySimulator/Blueprints/Grid/BP_TerrainGenerator.MaxHeight` _asbp_terrain_generator) 1.0 (`KismetMathLibrary.Conv_IntToDouble` (`/Game/StratagySimulator/Blueprints/Grid/BP_TerrainGenerator.TerrainDeep` _asbp_terrain_generator))) _fragmentsize_z))) :`End` (+ _returnvalue (`KismetMathLibrary.MakeVector` _returnvalue_2 _returnvalue_3)) :`Radius` 30.0 :`TraceChannel` "TraceTypeQuery1" :`bTraceComplex` true :`DrawDebugType` "ForDuration" :`bIgnoreSelf` false :`DrawTime` 15.0))
    (if _returnvalue_4
      (for _array_element _outhits
        (bind (_bblockinghit _binitialoverlap _time _distance _location _impactpoint _normal _impactnormal _physmat _hitactor _hitcomponent _hitbonename _hititem) (`GameplayStatics.BreakHitResult` _array_element))
        (bind (_success _result _terrain) (message `/Game/StratagySimulator/Blueprints/Grid/BP_TerrainConnectionInterface.GetImpactedComponent` _hitactor _hitcomponent))
        (if _success
          (bind (_fragmentsize_x_2 _fragmentsize_y_2 _fragmentsize_z_2) (`KismetMathLibrary.BreakVector` (`/Game/StratagySimulator/Blueprints/Grid/BP_TerrainGenerator.FragmentSize` _terrain)))
          (`|SpawnActorFromClass` "/Game/StratagySimulator/Blueprints/BP_ResourceContainerBase_Wood.BP_ResourceContainerBase_Wood_C" (`KismetMathLibrary.MakeTransform` (+ (.location (`InstancedStaticMeshComponent.GetInstanceTransform` _result _hititem true)) (`KismetMathLibrary.MakeVector` 0.0 0.0 (/ _fragmentsize_z_2 2.0))) (`KismetMathLibrary.MakeRotator` 0.0 0.0 (`KismetMathLibrary.RandomFloatInRange` -180.0 180.0))) "AlwaysSpawn" "OverrideRootScale" null null))))))

(fn `ClearResourceContainers`
  (for _array_element (`self.SpawnedResourceContainers`)
    (`Actor.K2_DestroyActor` _array_element))
  (`KismetArrayLibrary.Array_Clear` (`self.SpawnedResourceContainers`)))

(fn `GenerateResources`
  (locals (L_CurrentSpawnClass :type "/Game/StratagySimulator/Blueprints/BP_ResourceContainerBase Class Reference") (L_Terrain :type "/Game/StratagySimulator/Blueprints/Grid/BP_TerrainGenerator Object Reference") (L_Current_X :type Integer :default 0) (L_Current_Y :type Integer :default 0) (L_SpawnedPoints :type "Set of IntVector Structure") (L_Found :type Boolean :default false))
  (bind _l_terrain (`local.L_Terrain`))
  (bind _l_terrain_2 (`local.L_Terrain`))
  (bind _returnvalue (`Actor.K2_GetActorLocation` (`local.L_Terrain`)))
  (bind (_fragmentsize_x _fragmentsize_y _fragmentsize_z) (`KismetMathLibrary.BreakVector` (`/Game/StratagySimulator/Blueprints/Grid/BP_TerrainGenerator.FragmentSize` (`local.L_Terrain`))))
  (bind _returnvalue_2 (* (`local.L_Current_Y`) _fragmentsize_y))
  (bind _returnvalue_3 (* (`local.L_Current_X`) _fragmentsize_x))
  (`self.ClearResourceContainers`)
  (bind _asbp_terrain_generator (cast `/Game/StratagySimulator/Blueprints/Grid/BP_TerrainGenerator` (`self.GetOwner`)))
  (bind _output_get (set `local.L_Terrain` _asbp_terrain_generator))
  (`/Game/StratagySimulator/Blueprints/Grid/BP_TerrainGenerator.FillBiomes` _output_get)
  (bind _keys (`BlueprintMapLibrary.Map_Keys` (`self.Resources`)))
  (for _array_element _keys
    (set `local.L_CurrentSpawnClass` _array_element)
    (for _ (range (`BlueprintMapLibrary.Map_Find` (`self.Resources`) (`local.L_CurrentSpawnClass`)))
      (for _ (range (+ (`self.TriesToSpawnDebug`) 1))
        (set `local.L_Current_X` (`KismetMathLibrary.RandomIntegerInRange` 0 (`/Game/StratagySimulator/Blueprints/Grid/BP_TerrainGenerator.Width` _l_terrain)))
        (set `local.L_Current_Y` (`KismetMathLibrary.RandomIntegerInRange` 0 (`/Game/StratagySimulator/Blueprints/Grid/BP_TerrainGenerator.Length` _l_terrain)))
        (if (not (`BlueprintSetLibrary.Set_Contains` (`local.L_SpawnedPoints`) (make `IntVector` (`local.L_Current_X`) (`local.L_Current_Y`))))
          (`BlueprintSetLibrary.Set_Add` (`local.L_SpawnedPoints`) (make `IntVector` (`local.L_Current_X`) (`local.L_Current_Y`)))
          (set `local.L_Found` true)
          (break)))
      (if (`local.L_Found`)
        (bind (_outhits _returnvalue_4) (`KismetSystemLibrary.SphereTraceMulti` :`Start` (+ _returnvalue (`KismetMathLibrary.MakeVector` _returnvalue_3 _returnvalue_2 (* (+ (`/Game/StratagySimulator/Blueprints/Grid/BP_TerrainGenerator.MaxHeight` _l_terrain_2) 1.0 (`KismetMathLibrary.Conv_IntToDouble` (`/Game/StratagySimulator/Blueprints/Grid/BP_TerrainGenerator.TerrainDeep` _l_terrain_2))) _fragmentsize_z))) :`End` (+ _returnvalue (`KismetMathLibrary.MakeVector` _returnvalue_3 _returnvalue_2)) :`Radius` 30.0 :`TraceChannel` "TraceTypeQuery1" :`bTraceComplex` true :`DrawDebugType` "ForDuration" :`bIgnoreSelf` false :`DrawTime` 15.0))
        (if _returnvalue_4
          (for _array_element_2 _outhits
            (bind (_bblockinghit _binitialoverlap _time _distance _location _impactpoint _normal _impactnormal _physmat _hitactor _hitcomponent _hitbonename _hititem) (`GameplayStatics.BreakHitResult` _array_element_2))
            (bind (_success _result _terrain) (message `/Game/StratagySimulator/Blueprints/Grid/BP_TerrainConnectionInterface.GetImpactedComponent` _hitactor _hitcomponent))
            (if _success
              (bind (_fragmentsize_x_2 _fragmentsize_y_2 _fragmentsize_z_2) (`KismetMathLibrary.BreakVector` (`/Game/StratagySimulator/Blueprints/Grid/BP_TerrainGenerator.FragmentSize` _terrain)))
              (bind _returnvalue_5 (`|SpawnActorFromClass` (`local.L_CurrentSpawnClass`) (`KismetMathLibrary.MakeTransform` (+ (.location (`InstancedStaticMeshComponent.GetInstanceTransform` _result _hititem true)) (`KismetMathLibrary.MakeVector` 0.0 0.0 (/ _fragmentsize_z_2 2.0))) (`KismetMathLibrary.MakeRotator` 0.0 0.0 (`KismetMathLibrary.RandomFloatInRange` -180.0 180.0))) "AlwaysSpawn" "OverrideRootScale" null null))
              (`KismetArrayLibrary.Array_Add` (`self.SpawnedResourceContainers`) _returnvalue_5)
              (`KismetSystemLibrary.PrintString` "Hello")
              (break))))
        (else
          (return))))))