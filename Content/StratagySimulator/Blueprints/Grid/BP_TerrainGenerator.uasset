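; Grid terrain actor for a strategy simulator that builds randomized block landscapes from per-biome instanced static meshes.
; GenerateTerrain sums four randomized sine/cosine waves into column heights, then fills each column down to zero.
; GetRandomBiome picks each block's mesh by weighted random among biomes allowed at that height, with some restricted to non-surface or surface layers.
; Helpers identify hit biome components and sphere-trace rectangles, returning cells only if uniformly level.
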(event `self.ReceiveBeginPlay`
  (`self.FillBiomes`))

(fn `FillBiomes`
  (set `self.BiomeComponents` (`|MakeMap` "NewEnumerator0" (`self.GrassMesh`) "NewEnumerator1" (`self.MetalMesh`) "NewEnumerator2" (`self.ClayMesh`) "NewEnumerator3" (`self.StoneMesh`) "NewEnumerator4" (`self.SandMesh`) :!type "/Game/StratagySimulator/Blueprints/Grid/E_Biome Enum")))

(fn `GenerateTerrain`
  (locals (IsCos_3 :type Boolean) (IsCos_4 :type Boolean) (IsCos_2 :type Boolean) (IsCos_1 :type Boolean) (L_CurrentHeight_4 :type "Float (double-precision)") (L_CurrentHeight_3 :type "Float (double-precision)") (L_CurrentHeight_2 :type "Float (double-precision)") (L_CurrentHeight_1 :type "Float (double-precision)") (L_CurrentFrequency4 :type "Float (double-precision)") (L_CurrentFrequency3 :type "Float (double-precision)") (L_CurrentFrequency2 :type "Float (double-precision)") (L_CurrentFrequency1 :type "Float (double-precision)") (L_Current_X :type Integer) (L_Current_Y :type Integer) (L_Max_Z_By_XY :type Integer))
  (bind _returnvalue (`KismetMathLibrary.RandomBool`))
  (bind _l_currentfrequency2 (`local.L_CurrentFrequency2`))
  (bind _l_currentfrequency4 (`local.L_CurrentFrequency4`))
  (bind _l_currentfrequency3 (`local.L_CurrentFrequency3`))
  (bind (_fragmentsize_x _fragmentsize_y _fragmentsize_z) (`KismetMathLibrary.BreakVector` (`self.FragmentSize`)))
  (bind (_fragmentsize_x_2 _fragmentsize_y_2 _fragmentsize_z_2) (`KismetMathLibrary.BreakVector` (`self.FragmentSize`)))
  (bind _l_currentfrequency1 (`local.L_CurrentFrequency1`))
  (bind _returnvalue_2 (* (`local.L_Current_X`) _l_currentfrequency1))
  (bind _returnvalue_3 (`KismetMathLibrary.RandomFloatInRange` 0.0 (`self.MaxHeight`)))
  (bind _returnvalue_4 (* (`local.L_Current_X`) _l_currentfrequency4))
  (bind _returnvalue_5 (`KismetMathLibrary.RandomFloatInRange` 0.0 (`self.MaxFrequency`)))
  (bind _returnvalue_6 (* (`local.L_Current_Y`) _l_currentfrequency3))
  (bind _returnvalue_7 (`KismetMathLibrary.MakeVector` (* (`local.L_Current_X`) _fragmentsize_x) (* (`local.L_Current_Y`) _fragmentsize_y) (* (`local.L_Max_Z_By_XY`) _fragmentsize_z)))
  (bind _returnvalue_8 (* (* (`local.L_Current_Y`) _l_currentfrequency2) 0.88))
  (`self.FillBiomes`)
  (`InstancedStaticMeshComponent.ClearInstances` (`self.GrassMesh`))
  (`InstancedStaticMeshComponent.ClearInstances` (`self.ClayMesh`))
  (`InstancedStaticMeshComponent.ClearInstances` (`self.StoneMesh`))
  (`InstancedStaticMeshComponent.ClearInstances` (`self.SandMesh`))
  (`InstancedStaticMeshComponent.ClearInstances` (`self.MetalMesh`))
  ;[1 1 1] Setting random parameters
  (set `local.L_CurrentFrequency1` _returnvalue_5)
  (set `local.L_CurrentFrequency2` _returnvalue_5)
  (set `local.L_CurrentFrequency3` _returnvalue_5)
  (set `local.L_CurrentFrequency4` _returnvalue_5)
  (set `local.L_CurrentHeight_1` _returnvalue_3)
  (set `local.L_CurrentHeight_2` _returnvalue_3)
  (set `local.L_CurrentHeight_3` _returnvalue_3)
  (set `local.L_CurrentHeight_4` _returnvalue_3)
  (set `local.IsCos_1` _returnvalue)
  (set `local.IsCos_2` _returnvalue)
  (set `local.IsCos_3` _returnvalue)
  (set `local.IsCos_4` _returnvalue)
  (for _index (range (+ (`self.Width`) 1))
    (set `local.L_Current_X` _index)
    (for _index_2 (range (+ (`self.Length`) 1))
      (set `local.L_Current_Y` _index_2)
      (bind _output_get (set `local.L_Max_Z_By_XY` (+ (`KismetMathLibrary.Clamp` (`KismetMathLibrary.Round` (+ (* (`KismetMathLibrary.SelectFloat` (`KismetMathLibrary.DegSin` _returnvalue_2) (`KismetMathLibrary.DegCos` _returnvalue_2) (`local.IsCos_1`)) (`KismetMathLibrary.DegSin` (* (`local.L_Current_Y`) _l_currentfrequency1)) (`local.L_CurrentHeight_1`)) (* (`KismetMathLibrary.DegSin` (* (`local.L_Current_X`) _l_currentfrequency2)) (`KismetMathLibrary.SelectFloat` (`KismetMathLibrary.DegSin` _returnvalue_8) (`KismetMathLibrary.DegCos` _returnvalue_8) (`local.IsCos_2`)) (`local.L_CurrentHeight_2`)) (* (`KismetMathLibrary.DegSin` (* (* (`local.L_Current_X`) _l_currentfrequency3) 0.2)) (`KismetMathLibrary.SelectFloat` (`KismetMathLibrary.DegSin` _returnvalue_6) (`KismetMathLibrary.DegCos` _returnvalue_6) (`local.IsCos_3`)) (`local.L_CurrentHeight_3`)) (* (`KismetMathLibrary.SelectFloat` (`KismetMathLibrary.DegCos` _returnvalue_4) (`KismetMathLibrary.DegSin` _returnvalue_4) (`local.IsCos_4`)) (`KismetMathLibrary.DegSin` (* (* (`local.L_Current_Y`) _l_currentfrequency4) 0.9)) (`local.L_CurrentHeight_4`)))) 0 (`KismetMathLibrary.FTrunc` (`self.MaxHeight`))) (`self.TerrainDeep`))))
      (bind _value (`self.GetRandomBiome` _output_get true))
      (`InstancedStaticMeshComponent.AddInstance` _value (`KismetMathLibrary.MakeTransform` _returnvalue_7 (struct) (/ (`self.FragmentSize`) 100.0)))
      ;[1 1 1] add lower levels if max level on this XY-coords bigger than 0
      (if (> (`local.L_Max_Z_By_XY`) 0)
        (for _index_3 (range 1 (+ (`local.L_Max_Z_By_XY`) 1))
          (bind _value_2 (`self.GetRandomBiome` (- (`local.L_Max_Z_By_XY`) _index_3)))
          (`InstancedStaticMeshComponent.AddInstance` _value_2 (`KismetMathLibrary.MakeTransform` (- _returnvalue_7 (`KismetMathLibrary.MakeVector` 0.0 0.0 (* _index_3 _fragmentsize_z_2))) (struct) (/ (`self.FragmentSize`) 100.0))))))))

(fn `GetFragmentLocationsInRectangle`
  (params (Start :type "/Game/StratagySimulator/Blueprints/Grid/F_FragmentKey Structure") (End :type "/Game/StratagySimulator/Blueprints/Grid/F_FragmentKey Structure"))
  (returns (Success :type Boolean) (Result :type "Array of Vector Structure") (Places :type "Array of IntVector Structure"))
  (locals (L_ResultArray :type "Array of Vector Structure") (L_FragmentPlaces :type "Array of IntVector Structure") (L_FragmentWorldLocation :type "Vector Structure" :default (0.0 0.0 0.0)) (L_FragmrntPositionOnGrid :type "IntVector Structure") (L_RelativeHeight :type "Float (double-precision)" :default 0.0) (L_X_Iterator :type Integer) (L_Y_Iterator :type Integer) (L_Found :type Boolean :default false))
  (bind (_fragmentsize_x _fragmentsize_y _fragmentsize_z) (`KismetMathLibrary.BreakVector` (`self.FragmentSize`)))
  (bind (_fragmentsize_x_2 _fragmentsize_y_2 _fragmentsize_z_2) (`KismetMathLibrary.BreakVector` (`self.FragmentSize`)))
  (bind _l_resultarray (`local.L_ResultArray`))
  (bind (_fragmentsize_x_3 _fragmentsize_y_3) (`KismetMathLibrary.BreakVector` (`self.FragmentSize`)))
  (bind _returnvalue (`KismetMathLibrary.Round` (/ (.x (.location (`InstancedStaticMeshComponent.GetInstanceTransform` End_ParentMesh_2_D9A5CFB6447CF8B51C916ABC27114609 End_FragmentIndex_5_0D0D8D814F1ED06F949912B84582A4B6 false))) _fragmentsize_x_2)))
  (bind _returnvalue_2 (`KismetMathLibrary.Round` (/ (.y (.location (`InstancedStaticMeshComponent.GetInstanceTransform` End_ParentMesh_2_D9A5CFB6447CF8B51C916ABC27114609 End_FragmentIndex_5_0D0D8D814F1ED06F949912B84582A4B6 false))) _fragmentsize_y_2)))
  (bind _returnvalue_3 (`KismetMathLibrary.Round` (/ (.x (.location (`InstancedStaticMeshComponent.GetInstanceTransform` Start_ParentMesh_2_D9A5CFB6447CF8B51C916ABC27114609 Start_FragmentIndex_5_0D0D8D814F1ED06F949912B84582A4B6 false))) _fragmentsize_x)))
  (bind _returnvalue_4 (`KismetMathLibrary.Round` (/ (.y (.location (`InstancedStaticMeshComponent.GetInstanceTransform` Start_ParentMesh_2_D9A5CFB6447CF8B51C916ABC27114609 Start_FragmentIndex_5_0D0D8D814F1ED06F949912B84582A4B6 false))) _fragmentsize_y)))
  (bind _returnvalue_5 (`KismetMathLibrary.Round` (/ (.z (.location (`InstancedStaticMeshComponent.GetInstanceTransform` Start_ParentMesh_2_D9A5CFB6447CF8B51C916ABC27114609 Start_FragmentIndex_5_0D0D8D814F1ED06F949912B84582A4B6 false))) _fragmentsize_z)))
  (if (== _returnvalue_5 (`KismetMathLibrary.Round` (/ (.z (.location (`InstancedStaticMeshComponent.GetInstanceTransform` End_ParentMesh_2_D9A5CFB6447CF8B51C916ABC27114609 End_FragmentIndex_5_0D0D8D814F1ED06F949912B84582A4B6 false))) _fragmentsize_z_2)))
    (set `local.L_RelativeHeight` (.z (.location (`InstancedStaticMeshComponent.GetInstanceTransform` Start_ParentMesh_2_D9A5CFB6447CF8B51C916ABC27114609 Start_FragmentIndex_5_0D0D8D814F1ED06F949912B84582A4B6 false))))
    (for _index (range (`KismetMathLibrary.Min` _returnvalue_3 _returnvalue) (+ (`KismetMathLibrary.Max` _returnvalue_3 _returnvalue) 1))
      (set `local.L_X_Iterator` _index)
      (for _index_2 (range (`KismetMathLibrary.Min` _returnvalue_4 _returnvalue_2) (+ (`KismetMathLibrary.Max` _returnvalue_4 _returnvalue_2) 1))
        (set `local.L_Y_Iterator` _index_2)
        (set `local.L_FragmrntPositionOnGrid` (make `IntVector` (`local.L_X_Iterator`) (`local.L_Y_Iterator`) _returnvalue_5))
        (set `local.L_FragmentWorldLocation` (+ (`KismetMathLibrary.MakeVector` (* (`local.L_X_Iterator`) _fragmentsize_x_3) (* (`local.L_Y_Iterator`) _fragmentsize_y_3) (`local.L_RelativeHeight`)) (`self.K2_GetActorLocation`)))
        (bind (_outhits _returnvalue_6) (`KismetSystemLibrary.SphereTraceMulti` :`Start` (+ (`local.L_FragmentWorldLocation`) (0.0 0.0 200.0)) :`End` (`local.L_FragmentWorldLocation`) :`Radius` 25.0 :`TraceChannel` "TraceTypeQuery1" :`bTraceComplex` true :`bIgnoreSelf` false))
        (if _returnvalue_6
          (set `local.L_Found` false)
          (for _array_element _outhits
            (bind (_bblockinghit _binitialoverlap _time _distance _location _impactpoint _normal _impactnormal _physmat _hitactor _hitcomponent _hitbonename _hititem) (`GameplayStatics.BreakHitResult` _array_element))
            (if (== _hitactor self)
              (bind _asinstanced_static_mesh_component (cast `InstancedStaticMeshComponent` _hitcomponent))
              (set `local.L_Found` true)
              (if (== (`local.L_RelativeHeight`) (.z (.location (`InstancedStaticMeshComponent.GetInstanceTransform` _asinstanced_static_mesh_component _hititem false))))
                (`KismetArrayLibrary.Array_Add` (`local.L_ResultArray`) (`local.L_FragmentWorldLocation`))
                (`KismetArrayLibrary.Array_Add` (`local.L_FragmentPlaces`) (`local.L_FragmrntPositionOnGrid`))
                (break)
                (else
                  (return false)))))
          (if (not (`local.L_Found`))
            (return false))
          (else
            (return false)))))
    (return (> (`KismetArrayLibrary.Array_Length` _l_resultarray) 0) _l_resultarray (`local.L_FragmentPlaces`))
    (else
      (return false))))

(fn `GetImpactedComponent`
  (params (Component :type "PrimitiveComponent Object Reference"))
  (returns (Success :type Boolean) (Result :type "InstancedStaticMeshComponent Object Reference") (Terrain :type "/Game/StratagySimulator/Blueprints/Grid/BP_TerrainGenerator Object Reference"))
  (bind _values (`BlueprintMapLibrary.Map_Values` (`self.BiomeComponents`)))
  (for _array_element _values
    (if (== (`local.Component`) _array_element)
      (return true _array_element self)))
  (return false null self))

(fn `GetRandomBiome`
  (params (Height :type Integer) (MaxHeight :type Boolean))
  (returns (Value :type "InstancedStaticMeshComponent Object Reference") (BiomeType :type "/Game/StratagySimulator/Blueprints/Grid/E_Biome Enum"))
  (locals (L_RandomizedFloat :type "Float (double-precision)" :default 0.0) (LWeights :type "Map of /Game/StratagySimulator/Blueprints/Grid/E_Biome Enum to Float (double-precision)") (L_SumOfWeights :type "Float (double-precision)" :default 0.0))
  (set `local.LWeights` (`self.BiomeWeight`))
  (bind _keys (`BlueprintMapLibrary.Map_Keys` (`self.BiomeAllowableHeight`)))
  (for _array_element _keys
    (bind _value (`BlueprintMapLibrary.Map_Find` (`self.BiomeAllowableHeight`) _array_element))
    (if (and (>= (break `/Game/StratagySimulator/Blueprints/Data/Structs/F_IntClamp` _value) 0) (>= (`.Max_6_44D473C047A2FB3B2E9C2C8C92534D27` (break `/Game/StratagySimulator/Blueprints/Data/Structs/F_IntClamp` _value)) 0))
      (if (not (`KismetMathLibrary.InRange_IntInt` (`local.Height`) (break `/Game/StratagySimulator/Blueprints/Data/Structs/F_IntClamp` _value) (`.Max_6_44D473C047A2FB3B2E9C2C8C92534D27` (break `/Game/StratagySimulator/Blueprints/Data/Structs/F_IntClamp` _value))))
        (`BlueprintMapLibrary.Map_Remove` (`local.LWeights`) _array_element :!label _label))
      (elif (not MaxHeight)
        (goto _label))))
  (set `local.L_RandomizedFloat` (`KismetMathLibrary.RandomFloat`))
  (bind _keys_2 (`BlueprintMapLibrary.Map_Keys` (`local.LWeights`)))
  (for _array_element_2 _keys_2
    (set `local.L_SumOfWeights` (+ (`local.L_SumOfWeights`) (`BlueprintMapLibrary.Map_Find` (`local.LWeights`) _array_element_2))))
  (bind _keys_3 (`BlueprintMapLibrary.Map_Keys` (`local.LWeights`)))
  (for _array_element_3 _keys_3
    (`BlueprintMapLibrary.Map_Add` (`local.LWeights`) _array_element_3 (/ (`BlueprintMapLibrary.Map_Find` (`local.LWeights`) _array_element_3) (`local.L_SumOfWeights`))))
  (set `local.L_SumOfWeights` 0.0)
  (bind _keys_4 (`BlueprintMapLibrary.Map_Keys` (`local.LWeights`)))
  (for _array_element_4 _keys_4
    (bind _output_get (set `local.L_SumOfWeights` (+ (`local.L_SumOfWeights`) (`BlueprintMapLibrary.Map_Find` (`local.LWeights`) _array_element_4))))
    (if (>= _output_get (`local.L_RandomizedFloat`))
      (return (`BlueprintMapLibrary.Map_Find` (`self.BiomeComponents`) _array_element_4) _array_element_4))))

(fn `RefreshBiomes`
  (for _index (range (enumcount `/Game/StratagySimulator/Blueprints/Grid/E_Biome`))
    (bind _returnvalue (cast `/Game/StratagySimulator/Blueprints/Grid/E_Biome` (`KismetMathLibrary.Conv_IntToByte` _index)))
    (`BlueprintMapLibrary.Map_Add` (`self.BiomeAllowableHeight`) _returnvalue)
    (`BlueprintMapLibrary.Map_Add` (`self.BiomeWeight`) _returnvalue)))

(fn `UserConstructionScript`)