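; BP_CitizenCreator is a spawner that populates the area around itself with randomly named BP_Citizen actors.
; On BeginPlay, it loops to spawn citizens at random horizontal offsets, then fetches each one's personality message, using short Delay retries while either is invalid.
; A randomly rolled sex, used only to pick the male or female first-name DataTable, precedes a random surname lookup, with both written into the personality's Name struct.
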(event `self.ReceiveBeginPlay`
  (bind _returnvalue (`KismetMathLibrary.RandomFloatInRange` -1000.0 1000.0))
  (for _ (range 11)
    (bind _returnvalue_2 (`|SpawnActorFromClass` "/Game/StratagySimulator/BP_Citizen.BP_Citizen_C" (`KismetMathLibrary.MakeTransform` (`KismetMathLibrary.MakeVector` (+ (.x (`self.K2_GetActorLocation`)) _returnvalue) (+ _returnvalue (.y (`self.K2_GetActorLocation`))) (.z (`self.K2_GetActorLocation`)))) "Undefined" "OverrideRootScale" null null))
    (`/Engine/EditorBlueprintResources/StandardMacros.IsValid` _returnvalue_2 :!label _label
      (:`Is Valid`
        (bind _result (message `/Game/StratagySimulator/BPI_Character.GetPersonality` _returnvalue_2))
        (`/Engine/EditorBlueprintResources/StandardMacros.IsValid` _result :!label _label_2
          (:`Is Valid`
            (switch `/Game/StratagySimulator/Blueprints/Data/Enums/E_Sex` (cast `/Game/StratagySimulator/Blueprints/Data/Enums/E_Sex` (`KismetMathLibrary.Conv_IntToByte` (`KismetMathLibrary.RandomIntegerInRange` 0 (- (enumcount `/Game/StratagySimulator/Blueprints/Data/Enums/E_Sex`) 1))))
              (:`NewEnumerator0`
                (bind _outrownames (`DataTableFunctionLibrary.GetDataTableRowNames` "/Game/StratagySimulator/Blueprints/Data/Tables/DT_MaleNames.DT_MaleNames"))
                (bind _returnvalue_3 (`|GetDataTableRow` "/Game/StratagySimulator/Blueprints/Data/Tables/DT_MaleNames.DT_MaleNames" (`KismetArrayLibrary.Array_Random` _outrownames))
                  (:`then`
                    (bind _name (`/Game/StratagySimulator/BP_PersonalityComponent.Name` _result))
                    (setmembers `/Game/StratagySimulator/Blueprints/Data/Structs/F_CharacterName` :`StructRef` _name :`FirstName` (`.Name_2_4E877DD4404E3FFA88A3DBB6AD22C4A8` (break `/Game/StratagySimulator/Blueprints/Data/Structs/F_NameData` _returnvalue_3))))))
              (:`NewEnumerator1`
                (bind _outrownames_2 (`DataTableFunctionLibrary.GetDataTableRowNames` "/Game/StratagySimulator/Blueprints/Data/Tables/DT_FemaleNames.DT_FemaleNames"))
                (bind _returnvalue_4 (`|GetDataTableRow` "/Game/StratagySimulator/Blueprints/Data/Tables/DT_FemaleNames.DT_FemaleNames" (`KismetArrayLibrary.Array_Random` _outrownames_2))
                  (:`then`
                    (setmembers `/Game/StratagySimulator/Blueprints/Data/Structs/F_CharacterName` :`StructRef` _name :`FirstName` (`.Name_2_4E877DD4404E3FFA88A3DBB6AD22C4A8` (break `/Game/StratagySimulator/Blueprints/Data/Structs/F_NameData` _returnvalue_4)))))))
            (bind _outrownames_3 (`DataTableFunctionLibrary.GetDataTableRowNames` "/Game/StratagySimulator/Blueprints/Data/Tables/DT_Surnames.DT_Surnames"))
            (bind _returnvalue_5 (`|GetDataTableRow` "/Game/StratagySimulator/Blueprints/Data/Tables/DT_Surnames.DT_Surnames" (`KismetArrayLibrary.Array_Random` _outrownames_3))
              (:`then`
                (setmembers `/Game/StratagySimulator/Blueprints/Data/Structs/F_CharacterName` :`StructRef` _name :`Surname` (`.Name_2_4E877DD4404E3FFA88A3DBB6AD22C4A8` (break `/Game/StratagySimulator/Blueprints/Data/Structs/F_NameData` _returnvalue_5))))))
          (:`Is Not Valid`
            (`KismetSystemLibrary.Delay` 0.2)
            (goto _label_2))))
      (:`Is Not Valid`
        (`KismetSystemLibrary.Delay` 0.2)
        (goto _label)))))

(fn `UserConstructionScript`)