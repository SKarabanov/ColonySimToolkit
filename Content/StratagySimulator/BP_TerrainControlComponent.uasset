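; Player controller component that lets the player drag-select a rectangle of terrain fragments under the cursor in the strategy simulator.
; StartSelection traces under the cursor, stores the hit mesh instance as the first fragment and spawns a BP_FragmentHighlite there.
; A looping timer re-traces to update the last fragment and feeds the highlight the locations from the terrain's rectangle query.
; EndSelection stops the timer, clears both fragments and destroys the highlight.
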(event `self.ReceiveBeginPlay`
  (bind _asplayer_controller (cast `PlayerController` (`self.GetOwner`))
    (:`then`
      (set `self.OwningController` _asplayer_controller))
    (:`CastFailed`
      (`KismetSystemLibrary.PrintString` (`KismetStringLibrary.Concat_StrStr` "Owning controller not found in " (`KismetSystemLibrary.GetDisplayName` self)) true true (struct :`R` 1.0 :`G` 0.019289 :`A` 1.0) 5.0))))

(fn `EndSelection`
  (`KismetSystemLibrary.K2_ClearAndInvalidateTimerHandle` (`self.SelectionTimerHandle`))
  (set `self.FirstSelectedFragment` (struct))
  (set `self.LastSelectedFragment` (struct))
  (`Actor.K2_DestroyActor` (`self.SelectionActor`))
  (set `self.SelectionActor` null))

(fn `SelectFragments`
  (locals (L_Terrain :type "/Game/StratagySimulator/Blueprints/Grid/BP_TerrainGenerator Object Reference"))
  (bind (_hitresult _returnvalue) (`PlayerController.GetHitResultUnderCursorByChannel` (`self.OwningController`) "TraceTypeQuery1" true))
  (bind (_bblockinghit _binitialoverlap _time _distance _location _impactpoint _normal _impactnormal _physmat _hitactor _hitcomponent _hitbonename _hititem) (`GameplayStatics.BreakHitResult` _hitresult))
  (if _returnvalue
    (bind (_success _result _terrain) (message `/Game/StratagySimulator/Blueprints/Grid/BP_TerrainConnectionInterface.GetImpactedComponent` _hitactor _hitcomponent))
    (if _success
      (set `self.LastSelectedFragment` (make `/Game/StratagySimulator/Blueprints/Grid/F_FragmentKey` _result _hititem))
      (bind _output_get (set `local.L_Terrain` _terrain))
      (bind (_success_2 _result_2) (`/Game/StratagySimulator/Blueprints/Grid/BP_TerrainGenerator.GetFragmentLocationsInRectangle` _output_get (`self.FirstSelectedFragment`) (`self.LastSelectedFragment`)))
      (if _success_2
        (`/Game/StratagySimulator/Blueprints/Grid/BP_FragmentHighlite.UpdateSelection` (`self.SelectionActor`) _result_2)))))

(fn `StartSelection`
  (bind (_firstselectedfragment_parentmesh _firstselectedfragment_fragmentindex) (break `/Game/StratagySimulator/Blueprints/Grid/F_FragmentKey` (`self.FirstSelectedFragment`)))
  (bind (_hitresult _returnvalue) (`PlayerController.GetHitResultUnderCursorByChannel` (`self.OwningController`) "TraceTypeQuery1" true))
  (bind (_bblockinghit _binitialoverlap _time _distance _location _impactpoint _normal _impactnormal _physmat _hitactor _hitcomponent _hitbonename _hititem) (`GameplayStatics.BreakHitResult` _hitresult))
  (if _returnvalue
    (bind (_success _result _terrain) (message `/Game/StratagySimulator/Blueprints/Grid/BP_TerrainConnectionInterface.GetImpactedComponent` _hitactor _hitcomponent))
    (if _success
      (set `self.FirstSelectedFragment` (make `/Game/StratagySimulator/Blueprints/Grid/F_FragmentKey` _result _hititem))
      (bind _returnvalue_2 (`|SpawnActorFromClass` "/Game/StratagySimulator/Blueprints/Grid/BP_FragmentHighlite.BP_FragmentHighlite_C" (`KismetMathLibrary.MakeTransform` (.location (`InstancedStaticMeshComponent.GetInstanceTransform` _firstselectedfragment_parentmesh _firstselectedfragment_fragmentindex true)) (.rotation (`InstancedStaticMeshComponent.GetInstanceTransform` _firstselectedfragment_parentmesh _firstselectedfragment_fragmentindex true))) "AlwaysSpawn" "OverrideRootScale" null (`/Game/StratagySimulator/Blueprints/Grid/BP_TerrainGenerator.FragmentSize` _terrain) null))
      (set `self.SelectionActor` _returnvalue_2)
      (bind _returnvalue_3 (`KismetSystemLibrary.K2_SetTimer` self "SelectFragments" 0.1 true))
      (set `self.SelectionTimerHandle` _returnvalue_3))))