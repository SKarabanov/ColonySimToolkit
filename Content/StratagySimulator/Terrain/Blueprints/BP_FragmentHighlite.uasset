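; BP_FragmentHighlite is a terrain actor that highlights selected fragments with instances of the EnableFragments instanced mesh.
; UpdateSelection diffs the incoming points against the previous selection, changing only what differs.
; New points get an instance scaled to FragmentSize and raised just above the fragment.
; Dropped points are removed by sphere-tracing at their location and using the hit item as the instance index.
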(fn `UpdateSelection`
  (params (SelectionPoints :type "Array of Vector Structure"))
  (locals (L_ActualVectors :type "Set of Vector Structure"))
  (bind (_fragmentsize_x _fragmentsize_y _fragmentsize_z) (`KismetMathLibrary.BreakVector` (`self.FragmentSize`)))
  (`BlueprintSetLibrary.Set_AddItems` (`local.L_ActualVectors`) SelectionPoints)
  (bind _result (`BlueprintSetLibrary.Set_Difference` (`local.L_ActualVectors`) (`self.OldVectors`)))
  (bind _result_2 (`BlueprintSetLibrary.Set_ToArray` _result))
  (for _array_element _result_2
    (bind (_returnvalue_x _returnvalue_y _returnvalue_z) (`KismetMathLibrary.BreakVector` (- _array_element (`self.K2_GetActorLocation`))))
    (`InstancedStaticMeshComponent.AddInstance` (`self.EnableFragments`) (`KismetMathLibrary.MakeTransform` (`KismetMathLibrary.MakeVector` _returnvalue_x _returnvalue_y (+ _returnvalue_z (+ (/ _fragmentsize_z 2.0) 5.0))) (struct) (/ (`self.FragmentSize`) 100.0))))
  (bind _result_3 (`BlueprintSetLibrary.Set_Difference` (`self.OldVectors`) (`local.L_ActualVectors`)))
  (bind _result_4 (`BlueprintSetLibrary.Set_ToArray` _result_3))
  (for _array_element_2 _result_4
    (bind (_outhits _returnvalue) (`KismetSystemLibrary.SphereTraceMulti` :`Start` (+ _array_element_2 (0.0 0.0 100.0)) :`End` (- _array_element_2 (0.0 0.0 2.0)) :`Radius` 50.0 :`TraceChannel` "TraceTypeQuery1" :`bIgnoreSelf` false))
    (if _returnvalue
      (for _array_element_3 _outhits
        (bind (_bblockinghit _binitialoverlap _time _distance _location _impactpoint _normal _impactnormal _physmat _hitactor _hitcomponent _hitbonename _hititem) (`GameplayStatics.BreakHitResult` _array_element_3))
        (if (== _hitcomponent (`self.EnableFragments`))
          (`InstancedStaticMeshComponent.RemoveInstance` (`self.EnableFragments`) _hititem)
          (break)))))
  (set `self.OldVectors` (`local.L_ActualVectors`)))

(fn `UserConstructionScript`)