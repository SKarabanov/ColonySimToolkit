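; BP_TaskManager is a singleton actor that holds the global task list for the strategy simulator and creates the main HUD on BeginPlay.
; Construction destroys every other instance of its class.
; Adding a task keeps entries unique and fires a new-task notification.
; TryToTakeTask finds a component's first priority type present in the list, but assigns the task at that priority's index rather than the matching task's, without removing it.
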(event `self.ReceiveBeginPlay`
  (bind _returnvalue (`|CreateWidget` "/Game/StratagySimulator/UI/WBP_MainHUD.WBP_MainHUD_C"))
  (`UserWidget.AddToViewport` _returnvalue 0))

(fn `AddTaskToGlobalList`
  (params (NewTask :type "/Game/StratagySimulator/TaskSystem/Blueprints/BP_Task_Base Object Reference"))
  (`KismetArrayLibrary.Array_AddUnique` (`self.GlobalTaskList`) NewTask)
  (`self.OnNewTaskAdded`))

(fn `RemoveTaskFromGlobalList`
  (params (Task :type "/Game/StratagySimulator/TaskSystem/Blueprints/BP_Task_Base Object Reference"))
  (`KismetArrayLibrary.Array_RemoveItem` (`self.GlobalTaskList`) Task))

(fn `SetSingltone`
  (bind _outactors (`GameplayStatics.GetAllActorsOfClass` (`GameplayStatics.GetObjectClass` self)))
  (for _array_element _outactors
    (if (!= _array_element self)
      (`self.K2_DestroyActor` _array_element))))

(fn `TryToTakeTask`
  (params (TaskComponent :type "/Game/StratagySimulator/TaskSystem/Blueprints/BP_LocalTaskComponent Object Reference"))
  (returns (Result :type Boolean))
  (locals (L_TypesArray :type "Array of /Game/StratagySimulator/TaskSystem/Enums/E_TaskType Enum"))
  (for (_array_element _array_index) (`self.GlobalTaskList`)
    (`KismetArrayLibrary.Array_Set` (`local.L_TypesArray`) _array_index (`/Game/StratagySimulator/TaskSystem/Blueprints/BP_Task_Base.Type` _array_element) true))
  (for (_array_element_2 _array_index_2) (`/Game/StratagySimulator/TaskSystem/Blueprints/BP_LocalTaskComponent.GetSortedPriorityArray` (`local.TaskComponent`))
    (if (`KismetArrayLibrary.Array_Contains` (`local.L_TypesArray`) _array_element_2)
      (set `/Game/StratagySimulator/TaskSystem/Blueprints/BP_LocalTaskComponent.CurrentTask` (`|GetArrayItem` (`self.GlobalTaskList`) _array_index_2) (`local.TaskComponent`))
      (return true)))
  (return false))

(fn `UserConstructionScript`
  (`self.SetSingltone`))